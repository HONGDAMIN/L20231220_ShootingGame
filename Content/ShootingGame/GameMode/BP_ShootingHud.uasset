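; BP_ShootingHud is the shooting game's HUD, which creates the on-screen widget and keeps its HP display current.
; On BeginPlay it binds to player 0's BP_ShootingPlyerState HP-update dispatcher, retrying on a short timer until the cast succeeds.
; Binding pushes the current HP with a hardcoded maximum.
; HP updates print a debug message and feed the widget's SetHp.
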(event `self.ReceiveBeginPlay`
  (bind _returnvalue (`|CreateWidget` "/Game/ShootingGame/Widget/ShootingHudWidget.ShootingHudWidget_C"))
  (bind _output_get (set `self.HudWidget` _returnvalue))
  (`UserWidget.AddToViewport` _output_get 0)
  (`self.Bind My Player State`))

(fn `Bind My Player State`
  (bind _asbp_shooting_plyer_state (cast `/Game/ShootingGame/GameMode/BP_ShootingPlyerState` (`Controller.PlayerState` (`GameplayStatics.GetPlayerController` 0)))
    (:`then`
      (add `/Game/ShootingGame/GameMode/BP_ShootingPlyerState.NewEventDispatcher_UpdateHP` _asbp_shooting_plyer_state (`|CreateDelegate` :!event `EventHpUpdate`))
      (`self.EventHpUpdate` (`/Game/ShootingGame/GameMode/BP_ShootingPlyerState.CurHP` _asbp_shooting_plyer_state) 100.0))
    (:`CastFailed`
      (`KismetSystemLibrary.K2_SetTimer` null "Bind My Player State" 0.01))))

(fn `EventHpUpdate`
  (params (CurHP :type "Float (double-precision)") (MaxHP :type "Float (double-precision)"))
  (`KismetSystemLibrary.PrintString` (`KismetStringLibrary.Concat_StrStr` "HUD_UpdateHP CurHp" (`KismetStringLibrary.Conv_DoubleToString` CurHP)) true true (struct :`G` 0.66 :`B` 1.0 :`A` 1.0) 60.0)
  (`/Game/ShootingGame/Widget/ShootingHudWidget.Set Hp` (`self.HudWidget`) CurHP MaxHP))

(fn `UserConstructionScript`)