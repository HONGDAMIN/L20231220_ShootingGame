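; Shooting game actor that moves its Sphere0 component back and forth or along a path while switched on.
; A timeline drives the sphere's relative location from a scaled ValueX track and replays from the start whenever it finishes.
; On BeginPlay it binds to an event dispatcher on a referenced Switch.
; EventOverlap takes a begin flag to start or stop the motion.
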(event `DoPlay`
  (bind (_direction _valuex) (`Timeline|Timeline_0` :!label _label)
    (:`Update`
      (`SceneComponent.K2_SetRelativeLocation` (`self.Sphere_0`) (* _valuex 100.0) false false))
    (:`Finished`
      (goto _label :!via `PlayFromStart`))))

(event `Do Stop`
  (goto _label :!via `Stop`))

(event `self.ReceiveBeginPlay`
  (add `/Game/ShootingGame/BP_Switch.NewEventDispatcher_Doplay` (`self.Switch`) (`|CreateDelegate` :!event `EventOverlap`)))

(fn `EventOverlap`
  (params (Isbegin :type Boolean))
  (if Isbegin
    (`self.DoPlay`)
    (else
      (`self.Do Stop`))))

(fn `UserConstructionScript`)