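; BP_MoveRotation is an actor in the shooting game whose static mesh spins while its IsPlay flag is set.
; Tick adds a fixed relative rotation on two axes each frame, without delta-time scaling.
; BeginPlay binds to a dispatcher on the referenced Switch.
; DoPlay turns the flag on, while EventOverlap sets it from a begin/end boolean, so it can also stop the spin.
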(event `self.ReceiveTick`
  (params (DeltaSeconds :type "Float (single-precision)"))
  (if (`self.IsPlay`)
    (`SceneComponent.K2_AddRelativeRotation` (`self.StaticMesh`) (struct :`Yaw` 1.0 :`Roll` 1.0) false false)))

(event `DoPlay`
  (set `self.IsPlay` true))

(event `self.ReceiveBeginPlay`
  (add `/Game/ShootingGame/BP_Switch.NewEventDispatcher_Doplay` (`self.Switch`) (`|CreateDelegate` :!event `EventOverlap`)))

(fn `EventOverlap`
  (params (Isbegin :type Boolean))
  (set `self.IsPlay` Isbegin))

(fn `UserConstructionScript`)